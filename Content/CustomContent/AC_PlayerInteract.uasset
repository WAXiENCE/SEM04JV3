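; Actor component for the first-person character that finds interactable objects in the player's line of sight.
; On BeginPlay it casts its owner to BP_FirstPersonCharacter and caches it as PlayerRef.
; Its LineTrace function traces the Visibility channel forward from the camera over a given length, with debug drawing on.
; It returns the hit actor only if that actor implements BPI_Interactable, and does not trigger the interaction itself.
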(event `self.ReceiveBeginPlay`
  (bind _asbp_first_person_character (cast `/Game/FirstPerson/Blueprints/BP_FirstPersonCharacter` (`self.GetOwner`)))
  (set `self.PlayerRef` _asbp_first_person_character))

(fn `LineTrace`
  (params (Length :type "Float (double-precision)" :default 250.0))
  (returns (HitActor :type "Actor Object Reference"))
  (bind _firstpersoncamera (`/Game/FirstPerson/Blueprints/BP_FirstPersonCharacter.FirstPersonCamera` (`self.PlayerRef`)))
  (bind _returnvalue (`SceneComponent.K2_GetComponentLocation` _firstpersoncamera))
  (bind _outhit (`KismetSystemLibrary.LineTraceSingle` :`Start` _returnvalue :`End` (+ _returnvalue (* (`SceneComponent.GetForwardVector` _firstpersoncamera) Length)) :`TraceChannel` "TraceTypeQuery1" :`DrawDebugType` "ForDuration"))
  (bind (_bblockinghit _binitialoverlap _time _distance _location _impactpoint _normal _impactnormal _physmat _hitactor) (`GameplayStatics.BreakHitResult` _outhit))
  (if (and (`KismetSystemLibrary.IsValid` _hitactor) (`KismetSystemLibrary.DoesImplementInterface` _hitactor "/Game/CustomContent/InteractionSystem/BPI_Interactable.BPI_Interactable_C"))
    (return _hitactor)))