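; BP_Door is an interactable door actor that swings open and closed when its Interact event fires.
; A closed-state flag picks the direction, playing an open or close sound and running the OpenCloseDoor timeline forward or in reverse.
; The timeline's alpha lerps the door mesh's relative yaw between shut and a quarter turn open.
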(event `/Game/CustomContent/InteractionSystem/BPI_Interactable.Interact`
  (params (Actor :type "Actor Object Reference"))
  (if (`self.IsDoorClosed`)
    (set `self.IsDoorClosed` false)
    (`GameplayStatics.PlaySound2D` "/Game/CustomContent/Sounds/S_DoorOpen_Cue.S_DoorOpen_Cue" 1.0 1.0 0.0 null null)
    (bind (_direction _alpha) (`Timeline|OpenCloseDoor` :!label _label)
      (:`Update`
        (`SceneComponent.K2_SetRelativeRotation` (`self.SM_Door`) (`KismetMathLibrary.MakeRotator` 0.0 0.0 (`KismetMathLibrary.Lerp` 0.0 90.0 _alpha)) false false)))
    (else
      (set `self.IsDoorClosed` true)
      (`GameplayStatics.PlaySound2D` "/Game/CustomContent/Sounds/S_DoorClose_Cue.S_DoorClose_Cue" 1.0 1.0 0.0 null null)
      (goto _label :!via `Reverse`))))

(fn `UserConstructionScript`)