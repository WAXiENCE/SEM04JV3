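; BP_LightSwitch is an interactable wall switch actor that toggles a referenced light on and off.
; On Interact, a FlipFlop tilts the Switch component between two opposite pitches or yaws and plays a 2D click sound.
; It then inverts the visibility of the assigned Light's component, if valid, independently of the switch's flip state.
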(event `/Game/CustomContent/InteractionSystem/BPI_Interactable.Interact`
  (params (Actor :type "Actor Object Reference"))
  (bind _switch (`self.Switch`))
  (bind _light (`self.Light`))
  (bind _lightcomponent (`Light.LightComponent` _light))
  (`|ExecutionSequence`
    (:`then_0`
      ; Flip le commutateur
      (`/Engine/EditorBlueprintResources/StandardMacros.FlipFlop`
        (:`A`
          (`SceneComponent.K2_SetRelativeRotation` _switch (struct :`Pitch` -10.0) false false))
        (:`B`
          (`SceneComponent.K2_SetRelativeRotation` _switch (struct :`Pitch` 10.0) false false)))
      (`GameplayStatics.PlaySound2D` "/Game/CustomContent/Sounds/S_LigthSwitch_Cue.S_LigthSwitch_Cue" 1.0 1.0 0.0 null null))
    (:`then_1`
      ; Allume/Éteint lumière
      (`/Engine/EditorBlueprintResources/StandardMacros.IsValid` _light
        (:`Is Valid`
          (if (`SceneComponent.bVisible` _lightcomponent)
            (`SceneComponent.SetVisibility` _lightcomponent false false)
            (else
              (`SceneComponent.SetVisibility` _lightcomponent true false))))))))

(fn `UserConstructionScript`)